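; Base missile actor for skills that damages what it hits and then removes itself.
; When its damage component begins an overlap, it tries to damage the other actor, activates the hit effect and deactivates the trail.
; It then destroys the damage component, regardless of whether damage landed, and destroys the actor after a short delay.
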(event OnComponentBeginOverlap(DamageComponent)
  (params (OverlappedComponent :type Primitive%20Component%20Object%20Reference) (OtherActor :type Actor%20Object%20Reference) (OtherComp :type Primitive%20Component%20Object%20Reference) (OtherBodyIndex :type Integer) (bFromSweep :type Boolean) (SweepResult :type Hit%20Result%20Structure%20%28by%20ref%29))
  (Default|TryDoDamage (Variables|Default|GetDamageComponent) OtherActor)
  (Components|Activation|Activate (Variables|Default|GetNS_Hit) false)
  (Components|Activation|Deactivate (Variables|Default|GetNS_Trail))
  (Components|DestroyComponent (Variables|Default|GetDamageComponent))
  (Utilities|FlowControl|Delay 1.0)
  (Actor|DestroyActor))

(fn ConstructionScript
  (|CallParentFunction))