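; Base beam skill actor that projects a beam along its forward vector up to Range and periodically damages what it hits.
; Every tick, a Visibility line trace sets the end point, flattened to actor height on a hit, to drive the beam particle variables and place the BeamHit effect.
; A looping DamageInterval timer, fired once at BeginPlay and cleared on Destroyed, re-traces and passes the hit actor to DamageComponent.
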(event EventBeginPlay
  (CallFunction|SetParticleEffectTargets)
  (CallFunction|DoBeamDamage)
  (bind _returnvalue (Utilities|Time|SetTimerbyFunctionName 0 "DoBeamDamage" (Variables|Default|GetDamageInterval) true))
  (Variables|Default|SetActiveTimerHandle _returnvalue))

(event EventDestroyed
  (Utilities|Time|ClearandInvalidateTimerbyHandle (Variables|Default|GetActiveTimerHandle)))

(event EventTick
  (params (DeltaSeconds :type Float%20%28single-precision%29))
  (CallFunction|SetParticleEffectTargets))

(fn ConstructionScript
  (|CallParentFunction))

(fn GetDefaultBeamEndPoint
  (bind _range (Variables|Default|GetRange))
  (return (+ (Transformation|GetActorLocation) (* (Transformation|GetActorForwardVector) (Math|Vector|MakeVector _range _range (.z (Transformation|GetActorLocation)))))))

(fn GetBeamEndPoint
  (bind (_outhit _returnvalue) (Collision|LineTraceByChannel (Transformation|GetActorLocation) (CallFunction|GetDefaultBeamEndPoint) "TraceTypeQuery1" false 0 "None"))
  (if _returnvalue
    (return (Math|Transform|MakeTransform (Math|Vector|MakeVector (.X (Class|KismetMathLibrary|BreakVector3f (.ImpactPoint (Collision|BreakHitResult _outhit)))) (.Y (Class|KismetMathLibrary|BreakVector3f (.ImpactPoint (Collision|BreakHitResult _outhit)))) (.z (Transformation|GetActorLocation))) (Math|Rotator|MakeRotator 0.0 0.0 (.yaw (Math|Rotator|MakeRotationfromAxes (.Normal (Collision|BreakHitResult _outhit)) "0, 0, 0" "0, 0, 0"))) "1.000000,1.000000,1.000000") (Math|Vector|MakeVector 0.0 0.0 0.0) 0.0 0.0 0.0 (Math|Rotator|MakeRotator 0.0 0.0 0.0) 0.0 0.0 0.0 "1.000000,1.000000,1.000000")
    (else
      (return (Math|Transform|MakeTransform (CallFunction|GetDefaultBeamEndPoint) (Math|Rotator|MakeRotator 0.0 0.0 (.yaw (.rotation (Transformation|GetActorTransform)))) "1.000000,1.000000,1.000000") "0, 0, 0" 0.0 0.0 0.0 (Math|Rotator|MakeRotator 0.0 0.0 0.0) 0.0 0.0 0.0 "1.000000,1.000000,1.000000"))))

(fn SetParticleEffectTargets
  (bind _beamendtransform (CallFunction|GetBeamEndPoint))
  (bind _output_get (LocalVariables|SetBeamEndPoint _beamendtransform))
  (Niagara|SetNiagaraVariable(Vector3) (Variables|Default|GetBeam) "TargetVector" (.location _output_get))
  (Transformation|SetWorldTransform (Variables|Default|GetBeamHit) (LocalVariables|GetBeamEndPoint) false false)
  (Niagara|SetNiagaraVariable(Float) (Variables|Default|GetBeam) "DistanceToTarget" (Math|Vector|VectorLength (- (.location (LocalVariables|GetBeamEndPoint)) (Transformation|GetActorLocation))))
  (Niagara|SetNiagaraVariable(Vector3) (Variables|Default|GetBeam) "Offset" (/ (- (Transformation|GetActorLocation) (.location (LocalVariables|GetBeamEndPoint))) "-2.000000,-2.000000,-2.000000"))
  (Niagara|SetNiagaraVariable(Vector3) (Variables|Default|GetBeam) "OrientationVector" (* (Math|Vector|Normalize (- (Transformation|GetActorLocation) (.location (LocalVariables|GetBeamEndPoint)))) "1.000000,1.000000,1.000000")))

(fn DoBeamDamage
  (bind _damagecomponent (Variables|Default|GetDamageComponent))
  (bind _outhit (Collision|LineTraceByChannel (Transformation|GetActorLocation) (CallFunction|GetDefaultBeamEndPoint) "TraceTypeQuery1" false 0 "None"))
  (Transformation|SetWorldLocation _damagecomponent (.location _outhit) false true)
  (Default|TryDoDamage _damagecomponent (.hitactor _outhit)))