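; BP_NatureEssence is a Nature Essence actor with a lootable component and two spheres that bob vertically.
; Tick plays MainBobTimeline, which restarts from the beginning whenever it finishes.
; Each timeline update adds local Z offsets scaled from one height track, with Sphere1 moving opposite to LootableComponent and Sphere2 at different magnitudes.
; The offsets are additive rather than absolute positions, and the construction script is empty.
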(event EventTick
  (params (DeltaSeconds :type Float%20%28single-precision%29))
  (bind _main_bob_height (Timeline|Main%20Bob%20Timeline Play)
    (:Update
      (Utilities|FlowControl|Sequence
        (:then_0
          (Transformation|AddLocalOffset (Variables|Default|GetLootableComponent) (Math|Vector|MakeVector 0.0 0.0 (* _main_bob_height 0.5)) false false))
        (:then_1
          (Transformation|AddLocalOffset (Variables|Default|GetSphere1) (Math|Vector|MakeVector 0.0 0.0 (* _main_bob_height -0.25)) false false))
        (:then_2
          (Transformation|AddLocalOffset (Variables|Default|GetSphere2) (Math|Vector|MakeVector 0.0 0.0 (* _main_bob_height 0.2)) false false))))
    (:Finished
      (Timeline|Main%20Bob%20Timeline PlayFromStart))))

(fn ConstructionScript)