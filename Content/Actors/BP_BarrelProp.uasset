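; BP_BarrelProp is a breakable barrel prop that shatters and drops loot when its health runs out.
; Its HealthComponent's depleted dispatcher triggers the break, followed by LootContainerComponent loot drop and actor destruction after a short delay.
; Breaking spawns a short-lived FS_MasterField at the last damage location to apply radial force for Chaos fracture, then disables overlap events on the geometry collection.
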(event Custom|OnBreakEvent
  (CallFunction|BreakBarrel)
  (Default|DropLoot (Variables|Default|GetLootContainerComponent))
  (Utilities|FlowControl|Delay 6.0)
  (Actor|DestroyActor))

(event EventBeginPlay
  (EventDispatchers|BindEventtoOnHealthDepletedDispatcher (Variables|Default|GetHealthComponent) (delegate Custom|OnBreakEvent)))

(fn ConstructionScript)

(fn BreakBarrel
  (Development|PrintString "ITS GONEEE!!!")
  (bind _returnvalue (Game|SpawnActorfromClass "/Engine/EditorResources/FieldNodes/FS_MasterField.FS_MasterField_C" (Math|Transform|MakeTransform (Variables|/Game/Components/HealthComponent.HealthComponent_C|GetLastDamageLocation (Variables|Default|GetHealthComponent)) "0, 0, 0" "1.000000,1.000000,1.000000") "Undefined" 0 0))
  (Variables|/Engine/EditorResources/FieldNodes/FS_MasterField.FS_MasterField_C|SetActivationType _returnvalue "NewEnumerator4")
  (Actor|SetLifeSpan _returnvalue 1.0)
  (Variables|/Engine/EditorResources/FieldNodes/FS_MasterField.FS_MasterField_C|SetRadial%20Magnitude _returnvalue 5e+03)
  (Default|CETrigger _returnvalue)
  (Variables|/Script/Engine.PrimitiveComponent|SetbGenerateOverlapEvents (Variables|Default|GetBP_BarrelProp_GeometryCollection) false))